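; BP_PlayerCharacter is the player character Blueprint, whose only live logic adds a crosshair HUD for the local player.
; On BeginPlay, it checks IsLocallyControlled, then creates WBP_Crosshair and adds it to the viewport.
; Unconnected leftover nodes hold an aim-down-sights FOV toggle and select-then-deploy logic for a Teleport ability, none of which runs.
; Overlap, Tick and the construction script are empty.
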(event EventBeginPlay
  (if (Pawn|IsLocallyControlled)
    (bind _returnvalue (UserInterface|CreateWidget "/Game/UI/WBP_Crosshair.WBP_Crosshair_C"))
    (UserInterface|Viewport|AddtoViewport _returnvalue 0)))

(event Collision|EventActorBeginOverlap
  (params (OtherActor :type Actor%20Object%20Reference)))

(event EventTick
  (params (DeltaSeconds :type Float%20%28single-precision%29)))

(event Input|ActionEvents|InputActionEAbility
  (params (Key :type Key%20Structure :default "None")))

(fn ConstructionScript)