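; Player character Blueprint (V2) that puts a crosshair on screen and carries a Health component.
; BeginPlay adds WBP_Crosshair to the viewport without a local-control check, while Tick prints current health for the locally controlled character as debug output.
; The OnHealthChanged handler is empty.
; Unconnected rifle spawn-and-attach logic never runs, and it sets CurrentWeapon to None instead of the spawned BP_Rifle.
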(event OnHealthChanged(Health)
  (params (HealthComp :type Health%20Component%20Object%20Reference) (Health :type Float%20%28single-precision%29) (HealthDelta :type Float%20%28single-precision%29) (DamageType :type Damage%20Type%20Object%20Reference) (InstigatedBy :type Controller%20Object%20Reference) (DamageCauser :type Actor%20Object%20Reference)))

(event EventBeginPlay
  (bind _returnvalue (UserInterface|CreateWidget "/Game/UI/WBP_Crosshair.WBP_Crosshair_C"))
  (UserInterface|Viewport|AddtoViewport _returnvalue 0))

(event Collision|EventActorBeginOverlap
  (params (OtherActor :type Actor%20Object%20Reference)))

(event EventTick
  (params (DeltaSeconds :type Float%20%28single-precision%29))
  (if (Pawn|IsLocallyControlled)
    (Development|PrintString (Utilities|String|ToString(Float) (Variables|/Script/Valorant.HealthComponent|GetCurrentHealth (Variables|Default|GetHealth))))))

(fn ConstructionScript)